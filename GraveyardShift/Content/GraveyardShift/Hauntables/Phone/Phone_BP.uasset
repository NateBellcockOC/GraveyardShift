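; A grabbable, physics-simulated hauntable phone that rings when dropped and can shatter for score.
; Dropping it reports a noise event for AI hearing, sets the anim Blueprint ringing, and runs a timeline pulsing emissive and light.
; Grabbing it silences the ring.
; Hit impulse thresholds trigger impact sound or, if previously grabbed, breakage: points go to the game instance, poof and shatter play, then the actor is destroyed.
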(event `self.ReceiveBeginPlay`
  (`AudioComponent.Stop` (`self.Telephone_V2_audio`)))

(event `self.ReceiveHit`
  (params (MyComp :type "PrimitiveComponent Object Reference") (Other :type "Actor Object Reference") (OtherComp :type "PrimitiveComponent Object Reference") (bSelfMoved :type Boolean) (HitLocation :type "Vector Structure") (HitNormal :type "Vector Structure") (NormalImpulse :type "Vector Structure") (Hit :type "HitResult Structure (by ref)"))
  (bind _skeletalmesh (`self.SkeletalMesh`))
  ;[0.02083 0.02083 0.02083] Plays Sound if Velocity is above Threshold
  (if (> (`KismetMathLibrary.VSize` NormalImpulse) (`self.ImpulseThreshold`))
    (`AudioComponent.Play` (`self.Impact_Cue`) 0.0))
  ;[0.005208 0.005208 0.005208] Checks if the object is moving fast enough to break
  (if (> (`KismetMathLibrary.VSize` NormalImpulse) (`self.BreakThreshold`))
    (if (`self.WasGrabd`)
      ;[1 1 1] Adds score and Breaks (Original Code)
      (bind _asmy_game_inst (cast `/Game/VRTemplate/Blueprints/MyGameInst` (`GameplayStatics.GetGameInstance`)))
      (`/Game/VRTemplate/Blueprints/MyGameInst.Scorepoints` _asmy_game_inst (`self.Score`))
      (`ActorComponent.Activate` (`self.PoofCloud_Big`) false)
      (`AudioComponent.Play` (`self.ShatterNoise_Cue`) 0.0)
      (`PrimitiveComponent.SetSimulatePhysics` _skeletalmesh false)
      (`SceneComponent.SetVisibility` _skeletalmesh false false)
      (`KismetSystemLibrary.Delay` 0.5)
      (`self.K2_DestroyActor`))
    (else
      (set `self.WasGrabd` false))))

(event `self.GrabComponent.OnDropped`
  (set `self.WasGrabd` true)
  (`self.Ring`))

(event `self.GrabComponent.OnGrabbed`
  (`AudioComponent.Play` (`self.PickupSound_V3_audio`) 0.0)
  (`self.Stop Ringing`))

(event `Ring`
  (bind _asphone_hauntable_anim_blueprint (cast `/Game/GraveyardShift/Hauntables/Phone/Phone_Hauntable_AnimBlueprint` (`SkeletalMeshComponent.GetAnimInstance` (`self.SkeletalMesh`))))
  (set `/Game/GraveyardShift/Hauntables/Phone/Phone_Hauntable_AnimBlueprint.isRinging` true _asphone_hauntable_anim_blueprint)
  (`AudioComponent.Play` (`self.Telephone_V2_audio`) 0.0)
  (`AISense_Hearing.ReportNoiseEvent` (`self.K2_GetActorLocation`) 1.0 (`GameplayStatics.GetPlayerPawn` 0) 0.0 "Sound")
  (bind (_direction _newtrack_0) (`Timeline|Light Blinking` :!label _label)
    (:`Update`
      (`MeshComponent.SetScalarParameterValueOnMaterials` (`self.SkeletalMesh`) "Emission" _newtrack_0)
      (`LightComponent.SetIntensity` (`self.Blinker Light`) (* _newtrack_0 10.0)))
    (:`Finished`
      (`MeshComponent.SetScalarParameterValueOnMaterials` (`self.SkeletalMesh`) "Emission" 0.0 :!label _label_2)
      (`LightComponent.SetIntensity` (`self.Blinker Light`) 0.0)
      (`AudioComponent.Stop` (`self.Telephone_V2_audio`))
      (goto _label :!via `Stop`))))

(event `Stop Ringing`
  (bind _asphone_hauntable_anim_blueprint (cast `/Game/GraveyardShift/Hauntables/Phone/Phone_Hauntable_AnimBlueprint` (`SkeletalMeshComponent.GetAnimInstance` (`self.SkeletalMesh`))))
  (set `/Game/GraveyardShift/Hauntables/Phone/Phone_Hauntable_AnimBlueprint.isRinging` false _asphone_hauntable_anim_blueprint)
  (goto _label_2))

(fn `UserConstructionScript`)