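; Hauntable printer prop that can be haunted into printing or smashed for score after being grabbed.
; Haunt lights its emissive material, runs animation and audio, reports a noise event, and spawns paper at the output socket through chained Delays, guarded by IsPrinting.
; Hit plays impact audio above one impulse threshold; above the break threshold, a grabbed printer scores, shatters and destroys itself, while softer hits clear the grab flag.
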(event `self.ReceiveHit`
  (params (MyComp :type "PrimitiveComponent Object Reference") (Other :type "Actor Object Reference") (OtherComp :type "PrimitiveComponent Object Reference") (bSelfMoved :type Boolean) (HitLocation :type "Vector Structure") (HitNormal :type "Vector Structure") (NormalImpulse :type "Vector Structure") (Hit :type "HitResult Structure (by ref)"))
  (bind _printer (`self.Printer`))
  ;[0.02083 0.02083 0.02083] Plays Sound if Velocity is above Threshold
  (if (> (`KismetMathLibrary.VSize` NormalImpulse) (`self.ImpulseThreshold`))
    (`AudioComponent.Play` (`self.Impact_Cue`) 0.0))
  ;[0.005208 0.005208 0.005208] Checks if the object is moving fast enough to break
  (if (> (`KismetMathLibrary.VSize` NormalImpulse) (`self.BreakThreshold`))
    (if (`self.WasGrabd`)
      ;[1 1 1] Adds score and Breaks (Original Code)
      (bind _asmy_game_inst (cast `/Game/VRTemplate/Blueprints/MyGameInst` (`GameplayStatics.GetGameInstance`)))
      (`/Game/VRTemplate/Blueprints/MyGameInst.Scorepoints` _asmy_game_inst (`self.Score`))
      (`AudioComponent.Play` (`self.ShatterNoise_Cue`) 0.0)
      (`PrimitiveComponent.SetSimulatePhysics` _printer false)
      (`SceneComponent.SetVisibility` _printer false false)
      (`KismetSystemLibrary.Delay` 0.5)
      (`self.K2_DestroyActor`))
    (else
      (set `self.WasGrabd` false))))

(event `Haunt`
  (bind _printingnoise_v3_audio (`self.PrintingNoise_V3_audio`))
  (bind _printer (`self.Printer`))
  (bind _returnvalue (`KismetMathLibrary.Conv_VectorToTransform` (`SceneComponent.GetSocketLocation` _printer (`SkinnedMeshComponent.GetSocketBoneName` _printer "output_jnt"))))
  (`MeshComponent.SetScalarParameterValueOnMaterials` (`self.Printer`) "Emission" 1.0)
  (if (not (`self.isPrinting`))
    (set `self.isPrinting` true)
    (bind _asprinter_hauntable_anim_bp (cast `/Game/GraveyardShift/Hauntables/Printer/Printer_Hauntable_AnimBP` (`SkeletalMeshComponent.GetAnimInstance` (`self.Printer`))))
    (set `/Game/GraveyardShift/Hauntables/Printer/Printer_Hauntable_AnimBP.isHaunting` true _asprinter_hauntable_anim_bp)
    (`AudioComponent.Play` _printingnoise_v3_audio 0.0)
    (`AISense_Hearing.ReportNoiseEvent` (`self.K2_GetActorLocation`) 1.0 (`GameplayStatics.GetPlayerPawn` 0) 0.0 "Sound")
    (`KismetSystemLibrary.Delay` 5.0)
    (`|SpawnActorFromClass` "/Game/GraveyardShift/Throwable_Objects/SheetOfPaper.SheetOfPaper_C" _returnvalue "AlwaysSpawn" "OverrideRootScale" null null)
    (`KismetSystemLibrary.Delay` 1.0)
    (`|SpawnActorFromClass` "/Game/GraveyardShift/Throwable_Objects/SheetOfPaper.SheetOfPaper_C" _returnvalue "AlwaysSpawn" "OverrideRootScale" null null)
    (`KismetSystemLibrary.Delay` 1.0)
    (`|SpawnActorFromClass` "/Game/GraveyardShift/Throwable_Objects/SheetOfPaper.SheetOfPaper_C" _returnvalue "AlwaysSpawn" "OverrideRootScale" null null)
    (`KismetSystemLibrary.Delay` 1.0)
    (`|SpawnActorFromClass` "/Game/GraveyardShift/Throwable_Objects/SheetOfPaper.SheetOfPaper_C" _returnvalue "AlwaysSpawn" "OverrideRootScale" null null)
    (`KismetSystemLibrary.Delay` 1.0)
    (`|SpawnActorFromClass` "/Game/GraveyardShift/Throwable_Objects/SheetOfPaper.SheetOfPaper_C" _returnvalue "AlwaysSpawn" "OverrideRootScale" null null)
    (`KismetSystemLibrary.Delay` 1.0)
    (`|SpawnActorFromClass` "/Game/GraveyardShift/Throwable_Objects/SheetOfPaper.SheetOfPaper_C" _returnvalue "AlwaysSpawn" "OverrideRootScale" null null)
    (`KismetSystemLibrary.Delay` 1.0)
    (`|SpawnActorFromClass` "/Game/GraveyardShift/Throwable_Objects/SheetOfPaper.SheetOfPaper_C" _returnvalue "AlwaysSpawn" "OverrideRootScale" null null)
    (`KismetSystemLibrary.Delay` 1.0)
    (`|SpawnActorFromClass` "/Game/GraveyardShift/Throwable_Objects/SheetOfPaper.SheetOfPaper_C" _returnvalue "AlwaysSpawn" "OverrideRootScale" null null)
    (`KismetSystemLibrary.Delay` 1.0)
    (`|SpawnActorFromClass` "/Game/GraveyardShift/Throwable_Objects/SheetOfPaper.SheetOfPaper_C" _returnvalue "AlwaysSpawn" "OverrideRootScale" null null)
    (`KismetSystemLibrary.Delay` 1.0)
    (`|SpawnActorFromClass` "/Game/GraveyardShift/Throwable_Objects/SheetOfPaper.SheetOfPaper_C" _returnvalue "AlwaysSpawn" "OverrideRootScale" null null)
    (`KismetSystemLibrary.Delay` 4.71)
    (`MeshComponent.SetScalarParameterValueOnMaterials` (`self.Printer`) "Emission" 0.0)
    (set `/Game/GraveyardShift/Hauntables/Printer/Printer_Hauntable_AnimBP.isHaunting` false _asprinter_hauntable_anim_bp)
    (`AudioComponent.Stop` _printingnoise_v3_audio)
    (set `self.isPrinting` false)))

(fn `UserConstructionScript`)